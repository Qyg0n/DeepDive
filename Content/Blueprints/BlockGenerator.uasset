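; Procedural block scatter actor that adds BlockCount static mesh components in its construction script.
; Random vectors from a seeded stream feed a homemade Perlin-style 3D noise, remapped to locations within ±Size and scales between block size limits.
; The noise's Gradient uses unseeded random values, so Seed does not fully determine the layout.
; An older grid-threshold loop is disconnected, and the event graph is empty.
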(event EventBeginPlay)

(event Collision|EventActorBeginOverlap
  (params (OtherActor :type Actor%20Object%20Reference)))

(event EventTick
  (params (DeltaSeconds :type Float%20%28single-precision%29)))

(fn ConstructionScript
  (bind _seed (Variables|Default|GetSeed))
  (bind _blockcount (Variables|Default|GetBlockCount))
  (bind _maxblocksize (Variables|Default|GetMaxBlockSize))
  (bind _minblocksize (Variables|Default|GetMinBlockSize))
  (bind _size (Variables|Default|GetSize))
  (bind _returnvalue (* _size -1.0))
  (bind (_x _y _z) (Math|Vector|BreakVector _size))
  (bind _output_get (Variables|Default|SetUsedSeed (select (== _seed 0) (Math|Random|RandomInteger 999999) _seed)))
  (bind _output_get_2 (Variables|Default|SetStream (Math|Random|MakeRandomStream _output_get)))
  (Class|KismetMathLibrary|ResetRandomStream _output_get_2)
  (for _index (range 1 _blockcount)
    (LocalVariables|SetTemp "0, 0, 0")
    (AddComponent|AddStaticMeshComponent false (Math|Transform|MakeTransform (Math|Vector|MakeVector (Math|Float|MapRangeClamped (CallFunction|3DPerlinNoise (* (* (/ _size _blockcount) _index) (Math|Random|RandomUnitVectorfromStream _output_get_2)) 1.0 1.0) -1.0 1.0 (.x _returnvalue) _x) (Math|Float|MapRangeClamped (CallFunction|3DPerlinNoise (* (* (/ _size _blockcount) _index) (Math|Random|RandomUnitVectorfromStream _output_get_2)) 1.0 1.0) -1.0 1.0 (.y _returnvalue) _y) (Math|Float|MapRangeClamped (CallFunction|3DPerlinNoise (* (* (/ _size _blockcount) _index) (Math|Random|RandomUnitVectorfromStream _output_get_2)) 1.0 1.0) -1.0 1.0 (.z _returnvalue) _z)) "0, 0, 0" (Math|Vector|MakeVector (Math|Float|MapRangeClamped (CallFunction|3DPerlinNoise (* (* (/ _size _blockcount) _index) (Math|Random|RandomUnitVectorfromStream _output_get_2)) 1.0 1.0) -1.0 1.0 _minblocksize _maxblocksize) (Math|Float|MapRangeClamped (CallFunction|3DPerlinNoise (* (* (/ _size _blockcount) _index) (Math|Random|RandomUnitVectorfromStream _output_get_2)) 1.0 1.0) -1.0 1.0 _minblocksize _maxblocksize) (Math|Float|MapRangeClamped (CallFunction|3DPerlinNoise (* (* (/ _size _blockcount) _index) (Math|Random|RandomUnitVectorfromStream _output_get_2)) 1.0 1.0) -1.0 1.0 _minblocksize _maxblocksize))))))

(fn Noise
  (params (Value :type Float%20%28single-precision%29))
  (return (Math|Vector|MakeVector (Class|KismetMathLibrary|PerlinNoise1D Value) (Class|KismetMathLibrary|PerlinNoise1D (Math|Float|Power Value 3.0)) (Class|KismetMathLibrary|PerlinNoise1D (Math|Float|Power Value 6.0)))))

(fn 3DPerlinNoise
  (params (In :type Vector) (Scale :type Float%20%28single-precision%29) (Amplitude :type Float%20%28single-precision%29))
  (bind (_x _y _z) (Math|Vector|BreakVector In))
  (bind _output_get (LocalVariables|SetL (Math|Conversions|ToVector(Float) (Class|KismetMathLibrary|FTruncVector (/ In (Math|Float|Max(Float) Scale 0.1))))))
  (LocalVariables|SetU (+ _output_get 1))
  (LocalVariables|SetD (CallFunction|Fade (- In _output_get)))
  (return (* (CallFunction|Interpolate (Math|Vector|MakeVector (CallFunction|Interpolate (Math|Vector|MakeVector (CallFunction|Interpolate (Math|Vector|MakeVector (CallFunction|Gradient (Math|Vector4|MakeVector4 (.x (LocalVariables|GetL)) (.y (LocalVariables|GetL)) (.z (LocalVariables|GetL)) 0.0) (Math|Vector4|MakeVector4 _x _y _z 0.0)) (CallFunction|Gradient (Math|Vector4|MakeVector4 (.x (LocalVariables|GetU)) (.y (LocalVariables|GetU)) (.z (LocalVariables|GetU)) 0.0) (Math|Vector4|MakeVector4 _x _y _z 0.0)) (.x (LocalVariables|GetD)))) (CallFunction|Interpolate (Math|Vector|MakeVector (CallFunction|Gradient (Math|Vector4|MakeVector4 (.x (LocalVariables|GetL)) (.y (LocalVariables|GetL)) (.z (LocalVariables|GetL)) 0.0) (Math|Vector4|MakeVector4 _x _y _z 0.0)) (CallFunction|Gradient (Math|Vector4|MakeVector4 (.x (LocalVariables|GetU)) (.y (LocalVariables|GetU)) (.z (LocalVariables|GetU)) 0.0) (Math|Vector4|MakeVector4 _x _y _z 0.0)) (.x (LocalVariables|GetD)))) (.y (LocalVariables|GetD)))) (CallFunction|Interpolate (Math|Vector|MakeVector (CallFunction|Interpolate (Math|Vector|MakeVector (CallFunction|Gradient (Math|Vector4|MakeVector4 (.x (LocalVariables|GetL)) (.y (LocalVariables|GetL)) (.z (LocalVariables|GetL)) 0.0) (Math|Vector4|MakeVector4 _x _y _z 0.0)) (CallFunction|Gradient (Math|Vector4|MakeVector4 (.x (LocalVariables|GetU)) (.y (LocalVariables|GetU)) (.z (LocalVariables|GetU)) 0.0) (Math|Vector4|MakeVector4 _x _y _z 0.0)) (.x (LocalVariables|GetD)))) (CallFunction|Interpolate (Math|Vector|MakeVector (CallFunction|Gradient (Math|Vector4|MakeVector4 (.x (LocalVariables|GetL)) (.y (LocalVariables|GetL)) (.z (LocalVariables|GetL)) 0.0) (Math|Vector4|MakeVector4 _x _y _z 0.0)) (CallFunction|Gradient (Math|Vector4|MakeVector4 (.x (LocalVariables|GetU)) (.y (LocalVariables|GetU)) (.z (LocalVariables|GetU)) 0.0) (Math|Vector4|MakeVector4 _x _y _z 0.0)) (.x (LocalVariables|GetD)))) (.y (LocalVariables|GetD)))) (.z (LocalVariables|GetD)))) Amplitude)))

(fn Fade
  (params (In :type Vector))
  (return (* (+ (* In (- (* In 6.0) 15.0)) 1e+01) In In In)))

(fn Interpolate
  (params (In :type Vector))
  (bind _returnvalue (Math|Trig|GetPI))
  (bind _returnvalue_2 (* (.z In) _returnvalue))
  (bind _returnvalue_3 (Math|Trig|Cos(Radians) _returnvalue_2))
  (bind _returnvalue_4 (- 1.0 _returnvalue_3))
  (bind _returnvalue_5 (* _returnvalue_4 0.5))
  (return (+ (* (.x In) (- 1.0 _returnvalue_5)) (* (.y In) _returnvalue_5))))

(fn Gradient
  (params (One :type Vector%204%20Structure) (Two :type Vector%204%20Structure))
  (bind (_x _y _z _w) (Math|Vector4|BreakVector4 Two))
  (bind (_x_2 _y_2 _z_2 _w_2) (Math|Vector4|BreakVector4 One))
  (bind _returnvalue (Math|Random|RandomUnitVector))
  (return (+ (* (- _x_2 _x) (.x _returnvalue)) (* (- _y_2 _y) (.y _returnvalue)) (* (- _z_2 _z) (.z _returnvalue)) (* (- _w_2 _w) (Math|Random|RandomFloat)))))