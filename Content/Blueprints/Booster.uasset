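; Booster is a ring actor that pushes the player's glider when a DeepDivePlayer overlaps its trigger box.
; The overlap applies an impulse along the glider's forward vector, scaled by BoostAmount, and spawns a wind sound attached to the ring.
; While that sound is valid, Tick sets its volume from the effects volume and BoostAmount, divided by the glider's distance to the booster.
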(event OnComponentBeginOverlap(CheckPointTriggerBox)
  (params (OverlappedComponent :type Primitive%20Component%20Object%20Reference) (OtherActor :type Actor%20Object%20Reference) (OtherComp :type Primitive%20Component%20Object%20Reference) (OtherBodyIndex :type Integer) (bFromSweep :type Boolean) (SweepResult :type Hit%20Result%20Structure%20%28by%20ref%29))
  (bind (__ _valid) (CallFunction|GetDeepDivePlayer))
  (bind _glider (Variables|/Game/Blueprints/DeepDivePlayer.DeepDivePlayer_C|GetGlider __))
  (if (== (Utilities|GetClass OtherActor) "/Game/Blueprints/DeepDivePlayer.DeepDivePlayer_C")
    (if _valid
      (Physics|AddImpulse _glider (* (Math|Vector|GetForwardVector _glider) (Variables|Default|GetBoostAmount)) "None" false)
      (bind _returnvalue (Audio|SpawnSoundAttached "/Game/Assets/Sounds/Wind_Bolt_5_Cue.Wind_Bolt_5_Cue" (Variables|Default|GetCheckPointRing) "None" "0, 0, 0" "0, 0, 0" "KeepRelativeOffset" false 1.0 1.0 0.1 0 0))
      (bind _output_get (Variables|Default|SetS _returnvalue)))))

(event EventBeginPlay)

(event Collision|EventActorBeginOverlap
  (params (OtherActor :type Actor%20Object%20Reference)))

(event EventTick
  (params (DeltaSeconds :type Float%20%28single-precision%29))
  (Utilities|IsValid (stale OnComponentBeginOverlap(CheckPointTriggerBox) _output_get)
    (:Is%20Valid
      (Audio|Components|Audio|SetVolumeMultiplier (stale OnComponentBeginOverlap(CheckPointTriggerBox) _output_get) (* (.Effects (CallFunction|Volume)) (/ (/ (Variables|Default|GetBoostAmount) 2e+04) (/ (Math|Vector|Distance(Vector) (Transformation|GetWorldLocation (Variables|/Game/Blueprints/DeepDivePlayer.DeepDivePlayer_C|GetGlider (.%20 (CallFunction|GetDeepDivePlayer)))) (Transformation|GetActorLocation)) 1e+02))) :!class /Script/Engine.AudioComponent))))

(fn ConstructionScript)