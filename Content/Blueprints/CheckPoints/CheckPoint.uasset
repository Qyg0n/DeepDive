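; Checkpoint actor that registers the player's first pass through its trigger box and signals it with a light change.
; When an exact DeepDivePlayer overlaps, it sets IsCompleted, turns the point light green, swaps four sphere materials and calls CheckpointReached on DeepDive_Gamemode.
; Reset calls the parent, then restores the orange light and original material, but does not itself clear IsCompleted.
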(event OnComponentBeginOverlap(CheckPointTriggerBox)
  (params (OverlappedComponent :type Primitive%20Component%20Object%20Reference) (OtherActor :type Actor%20Object%20Reference) (OtherComp :type Primitive%20Component%20Object%20Reference) (OtherBodyIndex :type Integer) (bFromSweep :type Boolean) (SweepResult :type Hit%20Result%20Structure%20%28by%20ref%29))
  (if (not (Variables|Default|GetisCompleted))
    (if (== (Utilities|GetClass OtherActor) "/Game/Blueprints/DeepDivePlayer.DeepDivePlayer_C")
      (Variables|Default|SetisCompleted true)
      (Rendering|Components|Light|SetLightColor (Variables|Default|GetPointLight) "(R=0.005087,G=1.000000,B=0.000000,A=1.000000)" true)
      (Rendering|Material|SetMaterial (Variables|Default|GetSphere) 0 "/Game/Assets/Materials/Light_CP_Inst1.Light_CP_Inst1")
      (bind _asdeep_dive_gamemode (Utilities|Casting|CastToDeepDive_Gamemode (Game|GetGameMode)))
      (Default|CheckpointReached _asdeep_dive_gamemode))))

(event EventReset
  (|CallParentFunction)
  (Rendering|Material|SetMaterial (Variables|Default|GetSphere) 0 "/Game/Assets/Materials/Light_CP_Inst.Light_CP_Inst")
  (Rendering|Components|Light|SetLightColor (Variables|Default|GetPointLight) "(R=1.000000,G=0.619608,B=0.000000,A=1.000000)" true))

(event Collision|EventActorBeginOverlap
  (params (OtherActor :type Actor%20Object%20Reference))
  (|CallParentFunction OtherActor) ; This node is disabled and will not be called.\nDrag off pins to build functionality.
)

(event EventTick
  (params (DeltaSeconds :type Float%20%28single-precision%29))
  (|CallParentFunction DeltaSeconds) ; This node is disabled and will not be called.\nDrag off pins to build functionality.
)

(fn ConstructionScript
  (|CallParentFunction))