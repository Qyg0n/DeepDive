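; Finish line checkpoint for the DeepDive game, which completes only after every other checkpoint has been reached.
; When the DeepDivePlayer enters its trigger box, it scans all CheckPointParent actors except itself for any incomplete one.
; If none remain, it marks itself completed and notifies DeepDive_Gamemode that a checkpoint was reached and the finish was crossed.
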(event OnComponentBeginOverlap(CheckPointTriggerBox)
  (params (OverlappedComponent :type Primitive%20Component%20Object%20Reference) (OtherActor :type Actor%20Object%20Reference) (OtherComp :type Primitive%20Component%20Object%20Reference) (OtherBodyIndex :type Integer) (bFromSweep :type Boolean) (SweepResult :type Hit%20Result%20Structure%20%28by%20ref%29))
  (if (not (Variables|Default|GetisCompleted))
    (if (== (Utilities|GetClass OtherActor) "/Game/Blueprints/DeepDivePlayer.DeepDivePlayer_C")
      (Variables|Default|SetOneOrMoreCPNotComplete false)
      (bind _outactors (Actor|GetAllActorsOfClass "/Game/Blueprints/CheckPoints/CheckPointParent.CheckPointParent_C"))
      (for _array_element _outactors
        (if (!= _array_element self)
          (if (not (Variables|/Game/Blueprints/CheckPoints/CheckPointParent.CheckPointParent_C|GetisCompleted _array_element))
            (Variables|Default|SetOneOrMoreCPNotComplete true))))
      (if (not (Variables|Default|GetOneOrMoreCPNotComplete))
        (Variables|Default|SetisCompleted true)
        (bind _asdeep_dive_gamemode (Utilities|Casting|CastToDeepDive_Gamemode (Game|GetGameMode)))
        (Default|CheckpointReached _asdeep_dive_gamemode)
        (Default|CrossedFinish _asdeep_dive_gamemode)))))

(event Collision|EventActorBeginOverlap
  (params (OtherActor :type Actor%20Object%20Reference))
  (|CallParentFunction OtherActor) ; This node is disabled and will not be called.\nDrag off pins to build functionality.
)

(event EventTick
  (params (DeltaSeconds :type Float%20%28single-precision%29))
  (|CallParentFunction DeltaSeconds) ; This node is disabled and will not be called.\nDrag off pins to build functionality.
)

(fn ConstructionScript
  (|CallParentFunction))