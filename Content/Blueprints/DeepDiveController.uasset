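; DeepDive player controller that flies the possessed player's physics-simulated Glider and handles pause, retry and menu requests through the game mode.
; Each tick it rotates the glider from roll, pitch and yaw input, then bends velocity toward its nose with speed-based damping.
; Holding wing-toggle or brake alters this flight model, with wing influence blended over time.
; The escape menu freezes physics and pauses the pre-game timer, restoring saved velocity on closing mid-flight.
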(event Custom|Close_Event_0
  (bind _returnvalue (Game|GetGameMode))
  (bind _asdeep_dive_gamemode (Utilities|Casting|CastToDeepDive_Gamemode _returnvalue))
  (bind _pregame (Variables|/Game/Blueprints/DeepDive_Gamemode.DeepDive_Gamemode_C|GetPreGame _asdeep_dive_gamemode))
  (Utilities|FlowControl|Sequence
    (:then_0
      (Widget|RemovefromParent (stale Input|KeyboardEvents|Escape _output_get))
      (Utilities|IsValid (Variables|/Game/UI/EscMenu.EscMenu_C|GetWidget (stale Input|KeyboardEvents|Escape _output_get))
        (:Is%20Valid
          (Default|Close (Variables|/Game/UI/EscMenu.EscMenu_C|GetWidget (stale Input|KeyboardEvents|Escape _output_get))))
        (:Is%20Not%20Valid
          _))
      (Variables|Default|SetEscMenu 0)
      (Variables|/Game/Blueprints/DeepDive_Gamemode.DeepDive_Gamemode_C|SetPauseGame _asdeep_dive_gamemode false))
    (:then_1
      (if _pregame
        (Utilities|Time|UnpauseTimerbyHandle (Variables|/Game/Blueprints/DeepDive_Gamemode.DeepDive_Gamemode_C|GetTimer _asdeep_dive_gamemode))))
    (:then_2
      (if _pregame
        _
        (else
          (Physics|SetSimulatePhysics (Variables|Default|GetGlider) true)
          (Physics|SetPhysicsLinearVelocity (Variables|Default|GetGlider) (Variables|Default|GetCurrentVelolcity) false "None")))
      (Variables|Default|SetbShowMouseCursor false))))

(event Custom|Retry_Event_0
  (Default|RetryLevel (.AsDeep%20Dive%20Gamemode (Utilities|Casting|CastToDeepDive_Gamemode (Game|GetGameMode))))
  (Widget|RemovefromParent (stale Input|KeyboardEvents|Escape _output_get))
  (Utilities|IsValid (Variables|/Game/UI/EscMenu.EscMenu_C|GetWidget (stale Input|KeyboardEvents|Escape _output_get))
    (:Is%20Valid
      (Default|Close (Variables|/Game/UI/EscMenu.EscMenu_C|GetWidget (stale Input|KeyboardEvents|Escape _output_get))))
    (:Is%20Not%20Valid
      _))
  (Variables|Default|SetEscMenu 0)
  (Variables|/Game/Blueprints/DeepDive_Gamemode.DeepDive_Gamemode_C|SetPauseGame (.AsDeep%20Dive%20Gamemode (Utilities|Casting|CastToDeepDive_Gamemode (Game|GetGameMode))) false))

(event Custom|Menu_Event_0
  (Default|ToMenu (.AsDeep%20Dive%20Gamemode (Utilities|Casting|CastToDeepDive_Gamemode (Game|GetGameMode))))
  (Widget|RemovefromParent (stale Input|KeyboardEvents|Escape _output_get))
  (Utilities|IsValid (Variables|/Game/UI/EscMenu.EscMenu_C|GetWidget (stale Input|KeyboardEvents|Escape _output_get))
    (:Is%20Valid
      (Default|Close (Variables|/Game/UI/EscMenu.EscMenu_C|GetWidget (stale Input|KeyboardEvents|Escape _output_get))))
    (:Is%20Not%20Valid
      _))
  (Variables|Default|SetEscMenu 0)
  (Variables|/Game/Blueprints/DeepDive_Gamemode.DeepDive_Gamemode_C|SetPauseGame (.AsDeep%20Dive%20Gamemode (Utilities|Casting|CastToDeepDive_Gamemode (Game|GetGameMode))) false))

(event EventTick
  (params (DeltaSeconds :type Float%20%28single-precision%29))
  (bind _returnvalue (Math|Vector|MakeVector 0.0 0.0 1.0))
  (bind _returnvalue_2 (Game|GetGameMode))
  (bind _returnvalue_3 (Input|AxisValues|GetInput_Pitch))
  (bind _returnvalue_4 (Input|AxisValues|GetInput_Roll))
  (bind _returnvalue_5 (Input|AxisValues|GetInput_Yaw))
  (bind _glider (Variables|Default|GetGlider))
  (bind _glider_2 (Variables|Default|GetGlider))
  (bind _returnvalue_6 (Math|Vector|GetForwardVector _glider_2))
  (bind _returnvalue_7 (Math|Vector|GetUpVector _glider))
  (bind _returnvalue_8 (Math|Vector|GetForwardVector _glider))
  (bind _asdeep_dive_gamemode (Utilities|Casting|CastToDeepDive_Gamemode _returnvalue_2))
  (bind _returnvalue_9 (Math|Vector|DotProduct _returnvalue_8 _returnvalue))
  (bind _returnvalue_10 (Math|Vector|DotProduct _returnvalue_7 _returnvalue))
  (bind _pregame (Variables|/Game/Blueprints/DeepDive_Gamemode.DeepDive_Gamemode_C|GetPreGame _asdeep_dive_gamemode))
  (bind _returnvalue_11 (Math|Float|Absolute(Float) _returnvalue_10))
  (Variables|Default|SetDelta%20Seconds DeltaSeconds)
  (Utilities|IsValid (Variables|Default|GetGlider)
    (:Is%20Valid
      (if (Math|Boolean|NORBoolean _pregame (Variables|/Game/Blueprints/DeepDive_Gamemode.DeepDive_Gamemode_C|GetPauseGame _asdeep_dive_gamemode))
        (Utilities|FlowControl|Sequence
          (:then_0
            (bind _returnvalue_12 (Physics|GetPhysicsLinearVelocity (Variables|Default|GetGlider) "None"))
            (bind _output_get (Variables|Default|SetCurrentVelolcity _returnvalue_12))
            (Variables|Default|SetSpeed (Math|Vector|VectorLength _output_get)))
          (:then_1
            (Transformation|AddLocalRotation (Variables|Default|GetGlider) (* (Math|Rotator|MakeRotator (* (Variables|Default|GetRoll) 1e+02 1.0) (* (Variables|Default|GetPitch) -1e+02 (Math|Float|Lerp 1.0 (Math|Float|MapRangeClamped (Variables|Default|GetSpeed) 1e+03 4e+03 1.0 0.5) (Variables|Default|GetHasWingFloat))) (* (Variables|Default|GetYaw) 1e+02 0.2)) (Variables|Default|GetDelta%20Seconds)) false false)
            (Utilities|FlowControl|Sequence
              (:then_0
                (Variables|Default|SetHasWingFloat (Math|Float|Lerp (Math|Float|Max(Float) (- (Variables|Default|GetHasWingFloat) (* 1e+01 (Variables|Default|GetDelta%20Seconds))) 0.0) (Math|Float|Min(Float) (+ (Variables|Default|GetHasWingFloat) (* (Math|Float|MapRangeClamped (Variables|Default|GetSpeed) 1e+03 5e+03 6.0 3.0) (Variables|Default|GetDelta%20Seconds))) 1.0) (Math|Conversions|ToFloat(Boolean) (Variables|Default|GetHasWing)))))
              (:then_1
                ;[1 1 1] Rotation Changes Fly Direction
                (Physics|SetPhysicsLinearVelocity (Variables|Default|GetGlider) (Math|Vector|Lerp(Vector) (Variables|Default|GetCurrentVelolcity) (* (Math|Vector|Lerp(Vector) (Variables|Default|GetCurrentVelolcity) (* _returnvalue_6 (Math|Vector|VectorLength (Variables|Default|GetCurrentVelolcity))) (* (Math|Float|Max(Float) _returnvalue_11 (Math|Float|Absolute(Float) (Math|Vector|DotProduct (Math|Vector|Normalize (Variables|Default|GetCurrentVelolcity)) _returnvalue_6))) (Math|Float|MapRangeClamped (Math|Vector|VectorLength (Variables|Default|GetCurrentVelolcity)) 5e+02 2e+03 0.0 0.2) (select (> _returnvalue_9 0.0) (Math|Float|MapRangeClamped _returnvalue_11 0.0 _returnvalue_9 0.0 (- 1.0 _returnvalue_9)) 1.0))) (Math|Float|MapRangeClamped (Variables|Default|GetSpeed) 1e+02 1e+04 (Math|Float|MapRangeClamped (Variables|Default|GetSpeed) 1e+03 5e+03 1.0 (Math|Float|MapRangeClamped (Math|Float|Max(Float) _returnvalue_11 (Math|Float|Absolute(Float) (Math|Vector|DotProduct (Math|Vector|Normalize (Variables|Default|GetCurrentVelolcity)) _returnvalue_6))) 0.999 0.0 1.0 0.99)) (Math|Float|MapRangeClamped (Math|Conversions|ToFloat(Boolean) (Variables|Default|GetBreak)) 1.0 0.0 (* (Math|Float|MapRangeClamped (Variables|Default|GetSpeed) 1e+03 5e+03 1.0 (Math|Float|MapRangeClamped (Math|Float|Max(Float) _returnvalue_11 (Math|Float|Absolute(Float) (Math|Vector|DotProduct (Math|Vector|Normalize (Variables|Default|GetCurrentVelolcity)) _returnvalue_6))) 0.999 0.0 1.0 0.99)) 0.99) (Math|Float|MapRangeClamped (Variables|Default|GetSpeed) 1e+03 5e+03 1.0 (Math|Float|MapRangeClamped (Math|Float|Max(Float) _returnvalue_11 (Math|Float|Absolute(Float) (Math|Vector|DotProduct (Math|Vector|Normalize (Variables|Default|GetCurrentVelolcity)) _returnvalue_6))) 0.999 0.0 1.0 0.99))))) (Variables|Default|GetHasWingFloat)) false "None"))))
          (:then_2
            (Utilities|FlowControl|Sequence
              (:then_0
                (if (== _returnvalue_4 0.0)
                  (Variables|Default|SetRoll (Input|AxisValues|GetController_Roll))
                  (else
                    (Variables|Default|SetRoll (Math|Float|Lerp (Variables|Default|GetRoll) _returnvalue_4 (* (Variables|Default|GetAlpha) (Variables|Default|GetDelta%20Seconds)))))))
              (:then_1
                (if (== _returnvalue_3 0.0)
                  (Variables|Default|SetPitch (Input|AxisValues|GetController_Pitch))
                  (else
                    (Variables|Default|SetPitch (Math|Float|Lerp (Variables|Default|GetPitch) _returnvalue_3 (* (Variables|Default|GetAlpha) (Variables|Default|GetDelta%20Seconds)))))))
              (:then_2
                (if (== _returnvalue_5 0.0)
                  (Variables|Default|SetYaw (Input|AxisValues|GetController_Yaw))
                  (else
                    (Variables|Default|SetYaw (Math|Float|Lerp (Variables|Default|GetYaw) _returnvalue_5 (* (Variables|Default|GetAlpha) (Variables|Default|GetDelta%20Seconds))))))))))
        (elif _pregame
          (Variables|Default|SetSpeed 0.0))))))

(event EventPossess
  (params (PossessedPawn :type Pawn%20Object%20Reference))
  (bind __ (CallFunction|GetCharacter))
  (Utilities|IsValid __
    (:Is%20Valid
      (Variables|Default|SetGlider (Variables|/Game/Blueprints/DeepDivePlayer.DeepDivePlayer_C|GetGlider __))
      (Variables|Default|SetHasWing true)
      (Variables|Default|SetBreak false))))

(event Input|ActionEvents|InputActionAction_Retry
  (params (Key :type Key%20Structure :default "None"))
  (bind _returnvalue (Game|GetGameMode))
  (bind _asdeep_dive_gamemode (Utilities|Casting|CastToDeepDive_Gamemode _returnvalue))
  (:Pressed
    (if (Math|Boolean|NORBoolean (Variables|/Game/Blueprints/DeepDive_Gamemode.DeepDive_Gamemode_C|GetPreGame _asdeep_dive_gamemode) (Variables|/Game/Blueprints/DeepDive_Gamemode.DeepDive_Gamemode_C|GetPauseGame _asdeep_dive_gamemode))
      (bind _asdeep_dive_gamemode_2 (Utilities|Casting|CastToDeepDive_Gamemode (Game|GetGameMode)))
      (Default|RetryLevel _asdeep_dive_gamemode_2))))

(event Input|ActionEvents|InputActionAction_ToggleWing
  (params (Key :type Key%20Structure :default "None"))
  (bind _returnvalue (Game|GetGameMode))
  (bind __ (CallFunction|GetDeepDivePlayer))
  (bind _asdeep_dive_gamemode (Utilities|Casting|CastToDeepDive_Gamemode _returnvalue))
  (:Pressed
    (if (Math|Boolean|NORBoolean (Variables|/Game/Blueprints/DeepDive_Gamemode.DeepDive_Gamemode_C|GetPreGame _asdeep_dive_gamemode) (Variables|/Game/Blueprints/DeepDive_Gamemode.DeepDive_Gamemode_C|GetPauseGame _asdeep_dive_gamemode))
      (if (Variables|/Game/Blueprints/DeepDive_Gamemode.DeepDive_Gamemode_C|GetPlaying _asdeep_dive_gamemode)
        (Variables|Default|SetHasWing false)
        (Default|DeactivateWIngs __))))
  (:Released
    (Variables|Default|SetHasWing true)
    (Default|ActivateWings __)))

(event Input|ActionEvents|InputActionAction_Break
  (params (Key :type Key%20Structure :default "None"))
  (bind _returnvalue (Game|GetGameMode))
  (bind _asdeep_dive_gamemode (Utilities|Casting|CastToDeepDive_Gamemode _returnvalue))
  (:Pressed
    (if (Math|Boolean|NORBoolean (Variables|/Game/Blueprints/DeepDive_Gamemode.DeepDive_Gamemode_C|GetPreGame _asdeep_dive_gamemode) (Variables|/Game/Blueprints/DeepDive_Gamemode.DeepDive_Gamemode_C|GetPauseGame _asdeep_dive_gamemode))
      (if (Variables|/Game/Blueprints/DeepDive_Gamemode.DeepDive_Gamemode_C|GetPlaying _asdeep_dive_gamemode)
        (Variables|Default|SetBreak true))))
  (:Released
    (Variables|Default|SetBreak false)))

(event Input|KeyboardEvents|Escape
  (params (Key :type Key%20Structure :default "None"))
  (bind _returnvalue (Game|GetGameMode))
  (bind _asdeep_dive_gamemode (Utilities|Casting|CastToDeepDive_Gamemode _returnvalue))
  (:Pressed
    (Utilities|IsValid (stale _output_get)
      (:Is%20Not%20Valid
        (bind _returnvalue_2 (UserInterface|CreateWidget "/Game/UI/EscMenu.EscMenu_C"))
        (UserInterface|Viewport|AddtoViewport _returnvalue_2 0)
        (bind _output_get (Variables|Default|SetEscMenu _returnvalue_2))
        (Variables|/Game/Blueprints/DeepDive_Gamemode.DeepDive_Gamemode_C|SetPauseGame _asdeep_dive_gamemode true)
        (EventDispatchers|AssignClose _returnvalue_2 (delegate Custom|Close_Event_0))
        (EventDispatchers|AssignRetry _returnvalue_2 (delegate Custom|Retry_Event_0))
        (EventDispatchers|AssignMenu _returnvalue_2 (delegate Custom|Menu_Event_0))
        (Variables|Default|SetbShowMouseCursor true)
        (Physics|SetSimulatePhysics (Variables|Default|GetGlider) false)
        (if (Variables|/Game/Blueprints/DeepDive_Gamemode.DeepDive_Gamemode_C|GetPreGame _asdeep_dive_gamemode)
          (Utilities|Time|PauseTimerbyHandle (Variables|/Game/Blueprints/DeepDive_Gamemode.DeepDive_Gamemode_C|GetTimer _asdeep_dive_gamemode)))))))

(event Input|KeyboardEvents|NumPadZero
  (params (Key :type Key%20Structure :default "None"))
  (bind _returnvalue (Game|GetGameMode))
  (bind _asdeep_dive_gamemode (Utilities|Casting|CastToDeepDive_Gamemode _returnvalue))
  (:Pressed
    (Utilities|IsValid (stale _output_get)
      (:Is%20Not%20Valid
        (bind _returnvalue_2 (UserInterface|CreateWidget "/Game/UI/EscMenu.EscMenu_C"))
        (UserInterface|Viewport|AddtoViewport _returnvalue_2 0)
        (bind _output_get (Variables|Default|SetEscMenu _returnvalue_2))
        (Variables|/Game/Blueprints/DeepDive_Gamemode.DeepDive_Gamemode_C|SetPauseGame _asdeep_dive_gamemode true)
        (EventDispatchers|AssignClose _returnvalue_2 (delegate Custom|Close_Event_0))
        (EventDispatchers|AssignRetry _returnvalue_2 (delegate Custom|Retry_Event_0))
        (EventDispatchers|AssignMenu _returnvalue_2 (delegate Custom|Menu_Event_0))
        (Variables|Default|SetbShowMouseCursor true)
        (Physics|SetSimulatePhysics (Variables|Default|GetGlider) false)
        (if (Variables|/Game/Blueprints/DeepDive_Gamemode.DeepDive_Gamemode_C|GetPreGame _asdeep_dive_gamemode)
          (Utilities|Time|PauseTimerbyHandle (Variables|/Game/Blueprints/DeepDive_Gamemode.DeepDive_Gamemode_C|GetTimer _asdeep_dive_gamemode)))))))

(fn ConstructionScript)

(fn GetCharacter
  (bind _asdeep_dive_player (Utilities|Casting|CastToDeepDivePlayer (Pawn|GetControlledPawn)))
  (return _asdeep_dive_player))