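; Player glider for Deep Dive, a physics-driven mesh that switches between open and closed wings.
; On play it attaches Niagara effects to both wing sockets and a looping-style wind sound, stopped on end play.
; Each tick points an arrow along velocity and scales wind volume by speed minus camera distance and the effects volume setting.
; Wing toggle events swap the static mesh, saving and restoring linear velocity to preserve momentum.
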(event Custom|ActivateWings
  (bind _glider (Variables|Default|GetGlider))
  (bind _returnvalue (Physics|GetPhysicsLinearVelocity _glider "None"))
  (bind _output_get (Variables|Default|SetVelocity _returnvalue))
  (Components|StaticMesh|SetStaticMesh _glider "/Game/Assets/Glider/Glider.Glider")
  (Physics|SetPhysicsLinearVelocity _glider _output_get false "None"))

(event Custom|DeactivateWIngs
  (bind _glider (Variables|Default|GetGlider))
  (bind _returnvalue (Physics|GetPhysicsLinearVelocity _glider "None"))
  (bind _output_get (Variables|Default|SetVelocity _returnvalue))
  (Components|StaticMesh|SetStaticMesh _glider "/Game/Assets/Glider/Glider_closed.Glider_closed")
  (Physics|SetPhysicsLinearVelocity _glider _output_get false "None"))

(event EventBeginPlay
  (bind _returnvalue (AddComponent|AddNiagaraComponent true (Math|Transform|MakeTransform "0, 0, 0")))
  (Transformation|AttachComponentToComponent _returnvalue (Variables|Default|GetGlider) "LeftWing" "SnapToTarget" "SnapToTarget" "SnapToTarget" true)
  (bind _returnvalue_2 (AddComponent|AddNiagaraComponent true (Math|Transform|MakeTransform "0, 0, 0")))
  (Transformation|AttachComponentToComponent _returnvalue_2 (Variables|Default|GetGlider) "RightWing" "SnapToTarget" "SnapToTarget" "SnapToTarget" true)
  (bind _returnvalue_3 (Audio|SpawnSoundAttached "/Game/Assets/Sounds/Heavy_Wind_1_Cue.Heavy_Wind_1_Cue" (Variables|Default|GetGlider) "None" "0, 0, 0" "0, 0, 0" "KeepRelativeOffset" false 1.0 1.0 0.0 0 0))
  (Variables|Default|SetSound _returnvalue_3))

(event Collision|EventActorBeginOverlap
  (params (OtherActor :type Actor%20Object%20Reference)))

(event EventTick
  (params (DeltaSeconds :type Float%20%28single-precision%29))
  (bind _glider (Variables|Default|GetGlider))
  (bind _returnvalue (Transformation|GetWorldLocation _glider))
  (bind _returnvalue_2 (Physics|GetPhysicsLinearVelocity (Variables|Default|GetGlider) "None"))
  (Transformation|SetWorldRotation (Variables|Default|GetArrow) (Math|Rotator|FindLookatRotation _returnvalue (+ _returnvalue _returnvalue_2)) false false)
  (bind _returnvalue_3 (Physics|GetPhysicsLinearVelocity (Variables|Default|GetGlider) "None"))
  (Audio|Components|Audio|SetVolumeMultiplier (Variables|Default|GetSound) (* (.Effects (CallFunction|Volume)) (Math|Float|MapRangeClamped (- (Math|Vector|VectorLength _returnvalue_3) (Math|Vector|Distance(Vector) (Transformation|GetWorldLocation (Variables|Default|GetCamera)) (Transformation|GetWorldLocation (Variables|Default|GetGlider)))) 0.0 2e+04 0.0 0.2)) :!class /Script/Engine.AudioComponent))

(event EventEndPlay
  (params (EndPlayReason :type EEndPlayReason%20Enum :default "Destroyed"))
  (bind _sound (Variables|Default|GetSound))
  (Utilities|IsValid _sound
    (:Is%20Valid
      (Audio|Components|Audio|Stop _sound))))

(fn ConstructionScript)