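; Game mode for DeepDive, a timed glider game, running the main menu, level flow and music.
; Menu and levels stream in and out, and the Playing flag decides whether respawns spawn the glider player or a placeholder pawn with menu.
; Retries reset checkpoints and freeze glider physics for a short pre-game delay.
; Checkpoint splits are compared to the saved run, which faster finishes overwrite before the level-complete screen offers retry, next or menu.
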(event Custom|LevelComplete
  (bind _returnvalue (Game|GetPlayerController 0))
  (bind _save (Variables|Default|GetSave))
  (bind _currentlevel (Variables|Default|GetCurrentLevel))
  (bind _times (Variables|/Game/Blueprints/Save.Save_C|GetTimes _save))
  (bind (_value _returnvalue_2) (Utilities|Map|Find _times _currentlevel))
  (bind _times_2 (Utilities|Struct|BreakRun _value))
  (bind _returnvalue_3 (Utilities|Array|LastIndex _times_2))
  (bind _output (Utilities|Array|Get(acopy) _times_2 _returnvalue_3))
  (Utilities|FlowControl|Sequence
    (:then_0
      (bind _output_get (Variables|Default|SetLevelCompleted true))
      (Transformation|DetachFromComponent (Variables|/Game/Blueprints/DeepDivePlayer.DeepDivePlayer_C|GetCamera (.%20 (CallFunction|GetDeepDivePlayer))) "KeepWorld" "KeepWorld" "KeepWorld" true)
      (Utilities|FlowControl|Delay 1.0)
      (if _output_get
        (bind _returnvalue_4 (UserInterface|CreateWidget "/Game/UI/LevelCompleted.LevelCompleted_C" 0 (Math|Boolean|NORBoolean (Variables|Default|GetFreeplay) (== (Variables|Default|GetCurrentLevel) (Variables|Default|GetMaxLevels))) (Variables|Default|GetCheckPointTimes) (select _returnvalue_2 _output (Math|Timespan|MakeTimespan 0))))
        (bind _output_get_2 (Variables|Default|SetLevelCompletedRef _returnvalue_4))
        (UserInterface|Viewport|AddtoViewport _output_get_2 0)
        (EventDispatchers|AssignRetry _output_get_2 (delegate Custom|Retry_Event_0))
        (EventDispatchers|AssignNext _output_get_2 (delegate Custom|Next_Event_0))
        (EventDispatchers|AssignMenu _output_get_2 (delegate Custom|Menu_Event_0))
        (Variables|/Script/Engine.PlayerController|SetbShowMouseCursor _returnvalue true)
        (Widget|RemovefromParent (Variables|Default|GetTimerWidgetRef))
        (Variables|Default|SetTimerWidgetRef 0)
        (Input|SetInputModeGameandUI _returnvalue _output_get_2 "DoNotLock" true)))
    (:then_1
      (if _returnvalue_2
        (if (> _output (Variables|Default|GetTime))
          (Utilities|Map|Add _times (Variables|Default|GetCurrentLevel) (Utilities|Struct|MakeRun (Variables|Default|GetCheckPointTimes)) :!label _label)
          (SaveGame|SaveGametoSlot _save "Save")
          (Audio|SpawnSoundAttached "/Game/Assets/Sounds/Win_sound_4_Cue.Win_sound_4_Cue" (Variables|/Game/Blueprints/DeepDivePlayer.DeepDivePlayer_C|GetCamera (.%20 (CallFunction|GetDeepDivePlayer))) "None" "0, 0, 0" "0, 0, 0" "KeepRelativeOffset" false (.Effects (CallFunction|Volume)) 1.0 0.0 0 0))
        (else
          (goto _label))))))

(event Custom|CrossedFinish
  (CallFunction|LevelComplete))

(event Custom|ToMenu
  (Game|UnloadStreamLevel(byName) (CallFunction|LevelName (Variables|Default|GetCurrentLevel)) false)
  (Variables|Default|SetPlaying false)
  (Class|GameplayStatics|LoadStreamLevelbySoftObjectPtr "/Game/Level/MainMenu.MainMenu" true false)
  (CallFunction|RespawnPlayer)
  (Utilities|IsValid (Variables|Default|GetTimerWidgetRef)
    (:Is%20Valid
      (Widget|RemovefromParent (Variables|Default|GetTimerWidgetRef))
      (Variables|Default|SetTimerWidgetRef 0))))

(event Custom|CustomEvent_0
  (Physics|SetSimulatePhysics (Variables|/Game/Blueprints/DeepDivePlayer.DeepDivePlayer_C|GetGlider (.%20 (CallFunction|GetDeepDivePlayer))) true)
  (Variables|Default|SetPreGame false))

(event Custom|UpdateMusicVolume
  (params (Volume :type Float%20%28single-precision%29))
  (Audio|Components|Audio|SetVolumeMultiplier (stale EventBeginPlay _returnvalue_3) (* Volume 0.3) :!class /Script/Engine.AudioComponent))

(event Custom|Level_Event_0
  (params (Index :type Integer))
  (CallFunction|LoadLevel Index))

(event Custom|RespawnPlayer
  (bind _returnvalue (Game|GetPlayerController 0))
  (Actor|DestroyActor (Pawn|GetControlledPawn _returnvalue))
  (Pawn|UnPossess _returnvalue)
  (Class|GameModeBase|RestartPlayeratPlayerStart _returnvalue (Class|GameModeBase|FindPlayerStart)))

(event Custom|CheckpointReached
  (bind _effects (CallFunction|Volume))
  (bind _returnvalue (Math|Timespan|MakeTimespan 0))
  (bind __ (CallFunction|GetDeepDivePlayer))
  (bind _currentlevel (Variables|Default|GetCurrentLevel))
  (bind _save (Variables|Default|GetSave))
  (bind _time (Variables|Default|GetTime))
  (bind _camera (Variables|/Game/Blueprints/DeepDivePlayer.DeepDivePlayer_C|GetCamera __))
  (bind _times (Variables|/Game/Blueprints/Save.Save_C|GetTimes _save))
  (bind (_value _returnvalue_2) (Utilities|Map|Find _times _currentlevel))
  (bind _returnvalue_3 (Utilities|Array|Add (Variables|Default|GetCheckPointTimes) _time))
  (Default|ShowTime (Variables|Default|GetTimerWidgetRef) _time (select _returnvalue_2 (Utilities|Array|Get(acopy) (Utilities|Struct|BreakRun _value) _returnvalue_3) _returnvalue))
  (if (or (> (select _returnvalue_2 (Utilities|Array|Get(acopy) (Utilities|Struct|BreakRun _value) _returnvalue_3) _returnvalue) _time) (== (select _returnvalue_2 (Utilities|Array|Get(acopy) (Utilities|Struct|BreakRun _value) _returnvalue_3) _returnvalue) _returnvalue))
    (Audio|SpawnSoundAttached "/Game/Assets/Sounds/Win_sound_14_Cue.Win_sound_14_Cue" _camera "None" "0, 0, 0" "0, 0, 0" "KeepRelativeOffset" false _effects 1.0 0.0 0 0)
    (else
      (Audio|SpawnSoundAttached "/Game/Assets/Sounds/Win_sound_2_Cue.Win_sound_2_Cue" _camera "None" "0, 0, 0" "0, 0, 0" "KeepRelativeOffset" false _effects 1.0 0.0 0 0))))

(event Custom|Retry%20Level
  (bind _returnvalue (Game|GetPlayerController 0))
  (bind _levelcompletedref (Variables|Default|GetLevelCompletedRef))
  (if (Variables|Default|GetPlaying)
    (CallFunction|RespawnPlayer)
    (Variables|Default|SetTime (Math|Timespan|MakeTimespan 0))
    (Utilities|Array|Clear (Variables|Default|GetCheckPointTimes))
    (Utilities|FlowControl|Sequence
      (:then_0
        (Utilities|IsValid _levelcompletedref
          (:Is%20Valid
            (Widget|RemovefromParent _levelcompletedref))))
      (:then_1
        (bind _outactors (Actor|GetAllActorsOfClass "/Game/Blueprints/CheckPoints/CheckPointParent.CheckPointParent_C"))
        (for _array_element _outactors
          (Default|Reset _array_element))
        (Variables|/Script/Engine.PlayerController|SetbShowMouseCursor _returnvalue false)
        (Input|SetInputModeGameandUI _returnvalue 0 "DoNotLock" true)
        (Variables|Default|SetLevelCompleted false)
        (Variables|Default|SetPlaying true)
        (Variables|Default|SetPreGame true)
        (Utilities|FlowControl|Sequence
          (:then_0
            (Utilities|IsValid (Variables|Default|GetTimerWidgetRef)
              (:Is%20Not%20Valid
                (bind _returnvalue_2 (UserInterface|CreateWidget "/Game/UI/GameUI.GameUI_C"))
                (bind _output_get (Variables|Default|SetTimerWidgetRef _returnvalue_2))
                (UserInterface|Viewport|AddtoViewport _output_get 0))))
          (:then_1
            (Physics|SetSimulatePhysics (Variables|/Game/Blueprints/DeepDivePlayer.DeepDivePlayer_C|GetGlider (.%20 (CallFunction|GetDeepDivePlayer))) false)
            (bind _returnvalue_3 (Utilities|Time|SetTimerbyEvent (delegate Custom|CustomEvent_0) 3.0))
            (Variables|Default|SetTimer _returnvalue_3)))))))

(event Custom|Retry_Event_0
  (CallFunction|RetryLevel)
  (Widget|RemovefromParent (stale Custom|LevelComplete _output_get_2)))

(event Custom|Next_Event_0
  (CallFunction|LoadLevel (+ (Variables|Default|GetCurrentLevel) 1))
  (Widget|RemovefromParent (stale Custom|LevelComplete _output_get_2)))

(event Custom|Menu_Event_0
  (CallFunction|ToMenu)
  (Widget|RemovefromParent (stale Custom|LevelComplete _output_get_2)))

(event Custom|LoadLevel
  (params (Index :type Integer))
  (bind _returnvalue (UserInterface|CreateWidget "/Game/UI/Loading.Loading_C"))
  (bind _output_get (Variables|Default|SetLoading _returnvalue))
  (UserInterface|Viewport|AddtoViewport _output_get 10)
  (Game|LoadStreamLevel(byName) (CallFunction|LevelName Index) true)
  (if (Variables|Default|GetPlaying)
    (Game|UnloadStreamLevel(byName) (CallFunction|LevelName (Variables|Default|GetCurrentLevel)) false)
    (else
      (Class|GameplayStatics|UnloadStreamLevelbySoftObjectPtr "/Game/Level/MainMenu.MainMenu" false)
      (Widget|RemovefromParent (Variables|Default|GetMainMenu))))
  (Variables|Default|SetCurrentLevel Index)
  (Variables|Default|SetPlaying true)
  (CallFunction|RetryLevel)
  (Variables|/Script/Engine.PlayerController|SetbShowMouseCursor (Game|GetPlayerController 0) false)
  (Widget|RemovefromParent (Variables|Default|GetLoading)))

(event EventBeginPlay
  (bind _returnvalue (SaveGame|LoadGamefromSlot "Settings"))
  (bind _assettings (Utilities|Casting|CastToSettings _returnvalue)
    (:then
      (Variables|Default|SetSettings _assettings))
    (:CastFailed
      (bind _returnvalue_2 (SaveGame|CreateSaveGameObject "/Game/Blueprints/Settings.Settings_C"))
      (Variables|Default|SetSettings _returnvalue_2)))
  (bind _returnvalue_3 (Audio|CreateSound2D "/Game/Assets/Sounds/Music.Music" 1.0 1.0 0.0 0))
  (Audio|Components|Audio|SetVolumeMultiplier _returnvalue_3 (* (.Music (CallFunction|Volume)) 0.3) :!class /Script/Engine.AudioComponent)
  (Audio|Components|Audio|Play _returnvalue_3 0.0))

(event EventTick
  (params (DeltaSeconds :type Float%20%28single-precision%29))
  (if (Math|Boolean|ANDBoolean (Variables|Default|GetPlaying) (not (Variables|Default|GetLevelCompleted)) (not (Variables|Default|GetPauseGame)) (not (Variables|Default|GetPreGame)))
    (Variables|Default|SetTime (+ (Variables|Default|GetTime) (Math|Timespan|MakeTimespan 0 0 0 0 (Math|Float|Truncate (* DeltaSeconds 1e+03)))))))

(event EventOnRestartPlayer
  (params (NewPlayer :type Controller%20Object%20Reference))
  (bind _returnvalue (Game|GetPlayerController 0))
  (|CallParentFunction NewPlayer)
  (if (not (Variables|Default|GetPlaying))
    (bind _outactors (Actor|GetAllActorsOfClass "/Script/Engine.CameraActor"))
    (Game|Player|SetViewTargetwithBlend _returnvalue (Utilities|Array|Get(acopy) _outactors) 0.0 "VTBlend_Linear" 0.0 false)
    (Variables|/Script/Engine.PlayerController|SetbShowMouseCursor _returnvalue true)
    (bind _returnvalue_2 (UserInterface|CreateWidget "/Game/UI/MainMenu.MainMenu_C" 0 (Variables|Default|GetMaxLevels)))
    (bind _output_get (Variables|Default|SetMainMenu _returnvalue_2))
    (UserInterface|Viewport|AddtoViewport _output_get 0)
    (EventDispatchers|AssignLevel _output_get (delegate Custom|Level_Event_0))
    (bind _returnvalue_3 (SaveGame|LoadGamefromSlot "Save"))
    (bind _assave (Utilities|Casting|CastToSave _returnvalue_3)
      (:then
        (Variables|Default|SetSave _assave))
      (:CastFailed
        (bind _returnvalue_4 (SaveGame|CreateSaveGameObject "/Game/Blueprints/Save.Save_C"))
        (Variables|Default|SetSave _returnvalue_4)))))

(fn ConstructionScript)

(fn SpawnDefaultPawnfor
  (params (NewPlayer :type Controller%20Object%20Reference) (StartSpot :type Actor%20Object%20Reference))
  (if (Variables|Default|GetPlaying)
    (bind _returnvalue (|CallParentFunction NewPlayer StartSpot))
    (bind _asdeep_dive_player (Utilities|Casting|CastToDeepDivePlayer _returnvalue)
      (:then
        (Transformation|SetWorldRotation (Variables|/Game/Blueprints/DeepDivePlayer.DeepDivePlayer_C|GetGlider _asdeep_dive_player) (Transformation|GetActorRotation StartSpot) false false))
      (:CastFailed
        _))
    (return _returnvalue)
    (else
      (bind _returnvalue_2 (Game|SpawnActorfromClass "/Script/Engine.Pawn" (Math|Transform|MakeTransform "0, 0, 0" "0, 0, 0" "0.000000,0.000000,0.000000") "Undefined" 0 0))
      (return _returnvalue_2))))

(fn FindPlayerStart
  (params (Player :type Controller%20Object%20Reference) (IncomingName :type String))
  (bind _outactors (Actor|GetAllActorsOfClass "/Script/Engine.PlayerStart"))
  (return (Utilities|Array|Get(acopy) _outactors)))