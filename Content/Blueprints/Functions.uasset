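; Blueprint function library of shared helpers for the DeepDive game.
; Time helpers format minutes, seconds and milliseconds as a string or text, and LevelName builds a level name from an index.
; Typed getters cast the first player's controller and pawn and the game mode to their DeepDive classes, each returning a validity flag.
; Volume reads effects and music levels from the game mode's settings.
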(fn TimetoString
  (params (Time :type Timespan%20Structure))
  (bind (_days _hours _minutes _seconds _milliseconds) (Math|Timespan|BreakTimespan Time))
  (return (Utilities|String|Append (Utilities|String|ToString(Text) (Utilities|Text|ToText(Integer) _minutes false true 2)) " : " (Utilities|String|ToString(Text) (Utilities|Text|ToText(Integer) _seconds false true 2)) " : " (Utilities|String|ToString(Text) (Utilities|Text|ToText(Integer) _milliseconds false true 3)))))

(fn TimetoText
  (params (Time :type Timespan%20Structure))
  (bind (_days _hours _minutes _seconds _milliseconds) (Math|Timespan|BreakTimespan Time))
  (return (Utilities|Text|FormatText "{Min} : {Sec} : {Mill}" (Utilities|Text|ToText(Integer) _minutes false true 2) (Utilities|Text|ToText(Integer) _seconds false true 2) (Utilities|Text|ToText(Integer) _milliseconds false true 3))))

(fn LevelName
  (params (Index :type Integer))
  (return (Utilities|String|StringToName (Utilities|String|BuildString(Integer) "" "Level" Index))))

(fn GetDeepDiveController
  (bind ___worldcontext (LocalVariables|Get__WorldContext))
  (bind _returnvalue (Game|GetPlayerController ___worldcontext))
  (bind (_asdeep_dive_controller _bsuccess) (Utilities|Casting|CastToDeepDiveController _returnvalue))
  (return _asdeep_dive_controller _bsuccess))

(fn GetDeepDivePlayer
  (bind ___worldcontext (LocalVariables|Get__WorldContext))
  (bind _returnvalue (Game|Player|GetPlayerPawn ___worldcontext))
  (bind (_asdeep_dive_player _bsuccess) (Utilities|Casting|CastToDeepDivePlayer _returnvalue))
  (return _asdeep_dive_player _bsuccess))

(fn GetDeepDiveGM
  (bind ___worldcontext (LocalVariables|Get__WorldContext))
  (bind _returnvalue (Game|GetGameMode ___worldcontext))
  (bind (_asdeep_dive_gamemode _bsuccess) (Utilities|Casting|CastToDeepDive_Gamemode _returnvalue))
  (return _asdeep_dive_gamemode _bsuccess))

(fn Volume
  (bind ___worldcontext (LocalVariables|Get__WorldContext))
  (bind __ (CallFunction|GetDeepDiveGM ___worldcontext))
  (bind _settings (Variables|/Game/Blueprints/DeepDive_Gamemode.DeepDive_Gamemode_C|GetSettings __))
  (return (Variables|/Game/Blueprints/Settings.Settings_C|GetEffects _settings) (Variables|/Game/Blueprints/Settings.Settings_C|GetMusic _settings)))