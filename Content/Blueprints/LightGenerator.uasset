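; LightGenerator is a construction-time placement Blueprint that spawns child actors along a spline, presumably lights given its name.
; The construction script divides the spline length by Distance and adds a child actor component at each interval from the start.
; Each component takes the spline's local-space location and rotation at that point, with a fixed, reduced uniform scale.
; The event graph holds no active logic.
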(event EventBeginPlay)

(event Collision|EventActorBeginOverlap
  (params (OtherActor :type Actor%20Object%20Reference)))

(event EventTick
  (params (DeltaSeconds :type Float%20%28single-precision%29)))

(fn ConstructionScript
  (bind _spline (Variables|Default|GetSpline))
  (bind _distance (Variables|Default|GetDistance))
  (for _index (range 0 (Math|Float|Truncate (/ (Spline|GetSplineLength _spline) _distance)))
    (AddComponent|AddChildActorComponent false (Math|Transform|MakeTransform (Spline|GetLocationatDistanceAlongSpline _spline (* _index _distance) "Local") (Spline|GetRotationatDistanceAlongSpline _spline (* _index _distance) "Local") "0.100000,0.100000,0.100000"))))